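; BP_LaneCars is a lane of looping traffic that fills itself with BP_Vehicle actors moving in one direction.
; On BeginPlay it picks a random speed and direction, then InitializeLane spawns a row of spaced vehicles from the matching spawn point, rotated to that heading.
; Overlap triggers at each end recycle vehicles by moving them back to the opposite spawn point instead of respawning them.
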(event `self.ReceiveBeginPlay`
  (set `self.Speed` (`KismetMathLibrary.RandomFloatInRange` 200.0 400.0))
  (set `self.GoesLeft` (`KismetMathLibrary.RandomBool`))
  (`self.InitializeLane`))

(event `self.VehicleDetect Left.OnComponentBeginOverlap`
  (params (OverlappedComponent :type "PrimitiveComponent Object Reference") (OtherActor :type "Actor Object Reference") (OtherComp :type "PrimitiveComponent Object Reference") (OtherBodyIndex :type Integer) (bFromSweep :type Boolean) (SweepResult :type "HitResult Structure (by ref)"))
  (if (`self.GoesLeft`)
    (bind _asbp_vehicle (cast `/Game/Blueprints/BP_Vehicle` OtherActor))
    (`SceneComponent.K2_SetWorldLocation` (`Actor.RootComponent` _asbp_vehicle) (`SceneComponent.K2_GetComponentLocation` (`self.SpawnPoint Right`)) false false)))

(event `self.VehicleDetect Right.OnComponentBeginOverlap`
  (params (OverlappedComponent :type "PrimitiveComponent Object Reference") (OtherActor :type "Actor Object Reference") (OtherComp :type "PrimitiveComponent Object Reference") (OtherBodyIndex :type Integer) (bFromSweep :type Boolean) (SweepResult :type "HitResult Structure (by ref)"))
  (if (not (`self.GoesLeft`))
    (bind _asbp_vehicle (cast `/Game/Blueprints/BP_Vehicle` OtherActor))
    (`SceneComponent.K2_SetWorldLocation` (`Actor.RootComponent` _asbp_vehicle) (`SceneComponent.K2_GetComponentLocation` (`self.SpawnPoint Left`)) false false)))

(fn `InitializeLane`
  (bind (_returnvalue_x _returnvalue_y _returnvalue_z) (`KismetMathLibrary.BreakVector` (`SceneComponent.K2_GetComponentLocation` (`self.SpawnPoint Left`))))
  (bind (_returnvalue_x_2 _returnvalue_y_2 _returnvalue_z_2) (`KismetMathLibrary.BreakVector` (`SceneComponent.K2_GetComponentLocation` (`self.SpawnPoint Right`))))
  (if (`self.GoesLeft`)
    (for _index (range 4)
      (bind _returnvalue (`|SpawnActorFromClass` "/Game/Blueprints/BP_Vehicle.BP_Vehicle_C" (`KismetMathLibrary.MakeTransform` (`KismetMathLibrary.MakeVector` (+ _returnvalue_x_2 (* _index (`self.Spacing`))) _returnvalue_y_2 _returnvalue_z_2)) "Undefined" "OverrideRootScale" null null))
      (set `/Game/Blueprints/BP_Vehicle.MoveSpeed` (`self.Speed`) _returnvalue)
      (`self.K2_SetActorRotation` _returnvalue (struct :`Yaw` 270.0) false))
    (else
      (for _index_2 (range 4)
        (bind _returnvalue_2 (`|SpawnActorFromClass` "/Game/Blueprints/BP_Vehicle.BP_Vehicle_C" (`KismetMathLibrary.MakeTransform` (`KismetMathLibrary.MakeVector` (- _returnvalue_x (* _index_2 (`self.Spacing`))) _returnvalue_y _returnvalue_z)) "Undefined" "OverrideRootScale" null null))
        (set `/Game/Blueprints/BP_Vehicle.MoveSpeed` (`self.Speed`) _returnvalue_2)
        (`self.K2_SetActorRotation` _returnvalue_2 (struct :`Yaw` 90.0) false)))))

(fn `UserConstructionScript`)