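; BP_PlayerCharacter is the player-controlled chicken, which moves in discrete hops in four world-axis directions.
; Each move input uses LaunchCharacter with forward and upward speeds, gated by IsStopped, a low-velocity check that blocks new hops while moving.
; Each direction also plays its own timeline that lerps the PlayerChicken component's world rotation along the shortest path to a fixed facing.
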(event `InputAction|MoveForward`
  (params (Key :type "Key Structure"))
  (bind _playerchicken (`self.PlayerChicken`))
  (:`Pressed`
    (bind _ismoving (`self.IsStopped`))
    (if _ismoving
      (`self.LaunchCharacter` (`KismetMathLibrary.MakeVector` 0.0 (`self.ForwardSpeed`) (`self.HopSpeed`)))
      (bind (_direction _newtrack_0) (`Timeline|Begin Anim` :!via `PlayFromStart`)
        (:`Update`
          (`SceneComponent.K2_SetWorldRotation` _playerchicken (`KismetMathLibrary.RLerp` (`SceneComponent.K2_GetComponentRotation` _playerchicken) (struct :`Yaw` 180.0) _newtrack_0 true) false false))))))

(event `InputAction|MoveBackward`
  (params (Key :type "Key Structure"))
  (bind _playerchicken (`self.PlayerChicken`))
  (:`Pressed`
    (bind _ismoving (`self.IsStopped`))
    (if _ismoving
      (`self.LaunchCharacter` (`KismetMathLibrary.MakeVector` 0.0 (* (`self.ForwardSpeed`) -1.0) (`self.HopSpeed`)))
      (bind (_direction _newtrack_0) (`Timeline|Timeline_0` :!via `PlayFromStart`)
        (:`Update`
          (`SceneComponent.K2_SetWorldRotation` _playerchicken (`KismetMathLibrary.RLerp` (`SceneComponent.K2_GetComponentRotation` _playerchicken) (struct) _newtrack_0 true) false false))))))

(event `InputAction|MoveLeft`
  (params (Key :type "Key Structure"))
  (bind _playerchicken (`self.PlayerChicken`))
  (:`Pressed`
    (bind _ismoving (`self.IsStopped`))
    (if _ismoving
      (`self.LaunchCharacter` (`KismetMathLibrary.MakeVector` (`self.ForwardSpeed`) 0.0 (`self.HopSpeed`)))
      (bind (_direction _newtrack_0) (`Timeline|Timeline_1` :!via `PlayFromStart`)
        (:`Update`
          (`SceneComponent.K2_SetWorldRotation` _playerchicken (`KismetMathLibrary.RLerp` (`SceneComponent.K2_GetComponentRotation` _playerchicken) (struct :`Yaw` 90.0) _newtrack_0 true) false false))))))

(event `InputAction|MoveRight`
  (params (Key :type "Key Structure"))
  (bind _playerchicken (`self.PlayerChicken`))
  (:`Pressed`
    (bind _ismoving (`self.IsStopped`))
    (if _ismoving
      (`self.LaunchCharacter` (`KismetMathLibrary.MakeVector` (* (`self.ForwardSpeed`) -1.0) 0.0 (`self.HopSpeed`)))
      (bind (_direction _newtrack_0) (`Timeline|Timeline_2` :!via `PlayFromStart`)
        (:`Update`
          (`SceneComponent.K2_SetWorldRotation` _playerchicken (`KismetMathLibrary.RLerp` (`SceneComponent.K2_GetComponentRotation` _playerchicken) (struct :`Yaw` 270.0) _newtrack_0 true) false false))))))

(fn `IsStopped`
  (returns (IsMoving :type Boolean))
  (return (< (`KismetMathLibrary.VSize` (`self.GetVelocity`)) 20.0)))

(fn `UserConstructionScript`)