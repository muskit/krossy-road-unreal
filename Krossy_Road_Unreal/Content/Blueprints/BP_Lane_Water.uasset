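; BP_Lane_Water is a water lane that kills the player character and recycles moving logs.
; Overlapping the TriggerKill volume calls Kill on BP_PlayerCharacter.
; Left and right detector volumes catch BP_WaterLog actors and move them, without sweep, to the teleport point on the opposite side, so the logs wrap around the lane.
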(event `self.Trigger Kill.OnComponentBeginOverlap`
  (params (OverlappedComponent :type "PrimitiveComponent Object Reference") (OtherActor :type "Actor Object Reference") (OtherComp :type "PrimitiveComponent Object Reference") (OtherBodyIndex :type Integer) (bFromSweep :type Boolean) (SweepResult :type "HitResult Structure (by ref)"))
  (bind _asbp_player_character (cast `/Game/Blueprints/BP_PlayerCharacter` OtherActor))
  (`/Game/Blueprints/BP_PlayerCharacter.Kill` _asbp_player_character))

(event `self.Log Detector Left.OnComponentBeginOverlap`
  (params (OverlappedComponent :type "PrimitiveComponent Object Reference") (OtherActor :type "Actor Object Reference") (OtherComp :type "PrimitiveComponent Object Reference") (OtherBodyIndex :type Integer) (bFromSweep :type Boolean) (SweepResult :type "HitResult Structure (by ref)"))
  (bind _asbp_water_log (cast `/Game/Blueprints/BP_WaterLog` OtherActor))
  (`SceneComponent.K2_SetWorldLocation` (`Actor.RootComponent` _asbp_water_log) (`SceneComponent.K2_GetComponentLocation` (`self.TP Point Right`)) false false))

(event `self.Log Detector Right.OnComponentBeginOverlap`
  (params (OverlappedComponent :type "PrimitiveComponent Object Reference") (OtherActor :type "Actor Object Reference") (OtherComp :type "PrimitiveComponent Object Reference") (OtherBodyIndex :type Integer) (bFromSweep :type Boolean) (SweepResult :type "HitResult Structure (by ref)"))
  (bind _asbp_water_log (cast `/Game/Blueprints/BP_WaterLog` OtherActor))
  (`SceneComponent.K2_SetWorldLocation` (`Actor.RootComponent` _asbp_water_log) (`SceneComponent.K2_GetComponentLocation` (`self.TP Point Left`)) false false))

(fn `UserConstructionScript`
  (`parent.UserConstructionScript`))