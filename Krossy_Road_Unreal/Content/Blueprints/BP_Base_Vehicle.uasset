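; BP_Base_Vehicle is a base vehicle actor that acts as a moving hazard, killing the player character on contact.
; While KeepMoving is set, Tick offsets the root along its local Y axis at MoveSpeed, scaled by delta time.
; Overlaps on the front, back, left and right colliders each cast to BP_PlayerCharacter and share one Kill call, which targets all four cast results.
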(event `self.ReceiveTick`
  (params (DeltaSeconds :type "Float (single-precision)"))
  (if (`self.KeepMoving`)
    (`SceneComponent.K2_AddLocalOffset` (`self.DefaultSceneRoot`) (`KismetMathLibrary.MakeVector` 0.0 (* DeltaSeconds (`self.MoveSpeed`))) false false)))

(event `self.ColliderFront.OnComponentBeginOverlap`
  (params (OverlappedComponent :type "PrimitiveComponent Object Reference") (OtherActor :type "Actor Object Reference") (OtherComp :type "PrimitiveComponent Object Reference") (OtherBodyIndex :type Integer) (bFromSweep :type Boolean) (SweepResult :type "HitResult Structure (by ref)"))
  (bind _asbp_player_character (cast `/Game/Blueprints/BP_PlayerCharacter` OtherActor))
  (`/Game/Blueprints/BP_PlayerCharacter.Kill` _asbp_player_character :!label _label)
  (`/Game/Blueprints/BP_PlayerCharacter.Kill` (stale `self.ColliderLeft.OnComponentBeginOverlap` _asbp_player_character))
  (`/Game/Blueprints/BP_PlayerCharacter.Kill` (stale `self.ColliderBack.OnComponentBeginOverlap` _asbp_player_character))
  (`/Game/Blueprints/BP_PlayerCharacter.Kill` (stale `self.ColliderRight.OnComponentBeginOverlap` _asbp_player_character)))

(event `self.ColliderBack.OnComponentBeginOverlap`
  (params (OverlappedComponent :type "PrimitiveComponent Object Reference") (OtherActor :type "Actor Object Reference") (OtherComp :type "PrimitiveComponent Object Reference") (OtherBodyIndex :type Integer) (bFromSweep :type Boolean) (SweepResult :type "HitResult Structure (by ref)"))
  (bind _asbp_player_character (cast `/Game/Blueprints/BP_PlayerCharacter` OtherActor))
  (goto _label))

(event `self.ColliderLeft.OnComponentBeginOverlap`
  (params (OverlappedComponent :type "PrimitiveComponent Object Reference") (OtherActor :type "Actor Object Reference") (OtherComp :type "PrimitiveComponent Object Reference") (OtherBodyIndex :type Integer) (bFromSweep :type Boolean) (SweepResult :type "HitResult Structure (by ref)"))
  (bind _asbp_player_character (cast `/Game/Blueprints/BP_PlayerCharacter` OtherActor))
  (goto _label))

(event `self.ColliderRight.OnComponentBeginOverlap`
  (params (OverlappedComponent :type "PrimitiveComponent Object Reference") (OtherActor :type "Actor Object Reference") (OtherComp :type "PrimitiveComponent Object Reference") (OtherBodyIndex :type Integer) (bFromSweep :type Boolean) (SweepResult :type "HitResult Structure (by ref)"))
  (bind _asbp_player_character (cast `/Game/Blueprints/BP_PlayerCharacter` OtherActor))
  (goto _label))

(fn `UserConstructionScript`)