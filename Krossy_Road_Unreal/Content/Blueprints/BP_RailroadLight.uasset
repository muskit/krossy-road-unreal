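; BP_RailroadLight is a railroad signal light that flashes two point lights alternately.
; On BeginPlay it starts a looping timer of about a third of a second that calls SwitchLight by name.
; SwitchLight flips a boolean and shows one light while hiding the other, so no Tick logic is needed.
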(event `self.ReceiveBeginPlay`
  (`KismetSystemLibrary.K2_SetTimer` null "SwitchLight" 0.33 true))

(fn `SwitchLight`
  (bind _output_get (set `self.WhichLight` (not (`self.WhichLight`))))
  (if _output_get
    (`SceneComponent.SetVisibility` (`self.PointLight`) true false)
    (`SceneComponent.SetVisibility` (`self.PointLight1`) false false)
    (else
      (`SceneComponent.SetVisibility` (`self.PointLight`) false false)
      (`SceneComponent.SetVisibility` (`self.PointLight1`) true false))))

(fn `UserConstructionScript`)