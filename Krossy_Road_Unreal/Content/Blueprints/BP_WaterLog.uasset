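; BP_WaterLog is a log actor, named as a water obstacle or platform, that slides steadily along its local X axis.
; Tick offsets the scene root by MoveSpeed scaled by delta time, with GoesLeft choosing positive X and otherwise negative.
; A random assignment of GoesLeft sits disconnected in the construction script, so this Blueprint never randomizes its direction.
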(event `self.ReceiveTick`
  (params (DeltaSeconds :type "Float (single-precision)"))
  (if (`self.GoesLeft`)
    (`SceneComponent.K2_AddLocalOffset` (`self.DefaultSceneRoot`) (`KismetMathLibrary.MakeVector` (* DeltaSeconds (`self.MoveSpeed`))) false false)
    (else
      (`SceneComponent.K2_AddLocalOffset` (`self.DefaultSceneRoot`) (`KismetMathLibrary.MakeVector` (* (* DeltaSeconds (`self.MoveSpeed`)) -1.0)) false false))))

(fn `UserConstructionScript`)