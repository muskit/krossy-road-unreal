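; Lane spawner that procedurally builds a chained strip of grass, road and water lanes.
; On BeginPlay it spawns a base lane and several groups; SpawnNextGroup alternates grass groups with random mixes of road groups and single water lanes.
; Road groups open with an unmarked lane followed by marked ones.
; Each new lane spawns at the previous lane's SpawnPoint component and receives a reference back to the spawner.
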(event `self.ReceiveBeginPlay`
  (`self.SpawnInitialLanes`))

(event `SpawnNextGroup`
  (`/Engine/EditorBlueprintResources/StandardMacros.FlipFlop`
    (:`A`
      (`self.SpawnGroupGrass`))
    (:`B`
      (for _ (range (+ (`KismetMathLibrary.RandomIntegerInRange` 1 5) 1))
        (`|MultiGate` true true
          (:`Out 1`
            (`self.SpawnGroupRoad` (`KismetMathLibrary.RandomIntegerInRange` 1 6)))
          (:`Out 2`
            (`self.SpawnLane` "/Game/Blueprints/BP_Lane_Water.BP_Lane_Water_C")))))))

(fn `SpawnGroupGrass`
  (if true
    (for _ (range (+ (`KismetMathLibrary.RandomIntegerInRange` 1 4) 1))
      (`self.SpawnLane` "/Game/Blueprints/BP_Lane_Grass.BP_Lane_Grass_C"))))

(fn `SpawnGroupRoad`
  (params (LaneCount :type Integer))
  (for _index (range (+ LaneCount 1))
    (if (== _index 0)
      (`self.SpawnLane` "/Game/Blueprints/BP_Lane_Road_Unmarked.BP_Lane_Road_Unmarked_C")
      (else
        (`self.SpawnLane` "/Game/Blueprints/BP_Lane_RoadMarked.BP_Lane_RoadMarked_C")))))

(fn `SpawnInitialLanes`
  (bind _returnvalue (`|SpawnActorFromClass` "/Game/Blueprints/BP_Base_Lane.BP_Base_Lane_C" (`KismetMathLibrary.MakeTransform` (0.0 0.0 0.0)) "Undefined" "OverrideRootScale" null null))
  (set `self.RearmostLane` _returnvalue)
  (set `self.LatestLane` _returnvalue)
  (for _ (range 4)
    (`self.SpawnNextGroup`)))

(fn `SpawnLane`
  (params (LaneType :type "/Game/Blueprints/BP_Base_Lane Class Reference"))
  (bind _returnvalue (`|SpawnActorFromClass` LaneType (`KismetMathLibrary.MakeTransform` (`SceneComponent.K2_GetComponentLocation` (`self.GetComponentByClass` (`self.LatestLane`) "/Game/Blueprints/SpawnPoint.SpawnPoint_C"))) "Undefined" "OverrideRootScale" null null))
  (bind _output_get (set `self.LatestLane` _returnvalue))
  (set `/Game/Blueprints/BP_Base_Lane.LaneSpawner` self _output_get))

(fn `UserConstructionScript`)