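; BP_LaneSpawner is an actor that builds and extends a chain of BP_Lane segments.
; On BeginPlay it spawns a first lane at the world origin, flags it as SpawnedNext, records it as RearmostLane, then chains a few more.
; SpawnNextLane places each new lane at the latest lane's SpawnPoint component.
; Each lane receives a reference back to the spawner, and the newest is tracked as LatestLane.
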(event `self.ReceiveBeginPlay`
  (`self.SpawnInitialLanes`))

(fn `SpawnInitialLanes`
  (bind _latestlane (`self.LatestLane`))
  (`self.SpawnLane` (0.0 0.0 0.0))
  (set `/Game/Blueprints/BP_Lane.SpawnedNext` true _latestlane)
  (set `self.RearmostLane` _latestlane)
  (for _ (range 4)
    (`self.SpawnNextLane`)))

(fn `SpawnLane`
  (params (Location :type "Vector Structure"))
  (bind _returnvalue (`|SpawnActorFromClass` "/Game/Blueprints/BP_Lane.BP_Lane_C" (`KismetMathLibrary.MakeTransform` Location) "Undefined" "OverrideRootScale" null null))
  (bind _output_get (set `self.LatestLane` _returnvalue))
  (set `/Game/Blueprints/BP_Lane.LaneSpawner` self _output_get))

(fn `SpawnNextLane`
  (`self.SpawnLane` (`SceneComponent.K2_GetComponentLocation` (`self.GetComponentByClass` (`self.LatestLane`) "/Game/Blueprints/SpawnPoint.SpawnPoint_C"))))

(fn `UserConstructionScript`)